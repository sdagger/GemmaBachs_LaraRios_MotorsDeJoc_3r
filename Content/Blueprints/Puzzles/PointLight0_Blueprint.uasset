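; Puzzle point light Blueprint that cycles its color through blue, red and green.
; CustomEvent_0 calls SwitchLight, which branches on Counter to set the next color and advance or wrap the counter.
; The blue step sets color through PointLightComponent, while red and green go through LightComponent.
; Each step prints a debug string, including a fallback message when Counter is out of range.
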(event `CustomEvent_0`
  (`self.SwitchLight`))

(fn `SwitchLight`
  (if (== (`self.counter`) 0)
    ;[1 1 1] set blue color
    (`LightComponent.SetLightColor` (`self.PointLightComponent`) (`KismetMathLibrary.Conv_ColorToLinearColor` (`self.colorBlue`)) true)
    (set `self.counter` 1)
    (`KismetSystemLibrary.PrintString` "light color blue")
    (elif (== (`self.counter`) 1)
      ;[1 1 1] set red color
      (`LightComponent.SetLightColor` (`self.LightComponent`) (`KismetMathLibrary.Conv_ColorToLinearColor` (`self.colorRed`)) true)
      (set `self.counter` 2)
      (`KismetSystemLibrary.PrintString` "light color red")
      (elif (== (`self.counter`) 2)
        ;[1 1 1] set green color
        (`LightComponent.SetLightColor` (`self.LightComponent`) (`KismetMathLibrary.Conv_ColorToLinearColor` (`self.colorGreen`)) true)
        (set `self.counter` 0)
        (`KismetSystemLibrary.PrintString` "light color green")
        (else
          (`KismetSystemLibrary.PrintString` "NO COLOR CHANGED"))))))

(fn `UserConstructionScript`)