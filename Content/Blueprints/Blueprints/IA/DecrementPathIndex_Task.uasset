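; Behavior tree task that steps an AI's path index backwards while it travels from the end of its path toward the start.
; It runs only when the blackboard direction is -1, decrementing the path index and succeeding while the result stays at zero or above.
; At the start of the path it flips the direction to 1 and fails, as it also does for any other direction.
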(event `self.ReceiveExecuteAI`
  (params (OwnerController :type "AIController Object Reference") (ControlledPawn :type "Pawn Object Reference"))
  (bind _bblackboard_direction (`self.BBlackboard_Direction`))
  (bind _returnvalue (- (`BTFunctionLibrary.GetBlackboardValueAsInt` (`self.BBlackboard_PathIndex`)) 1))
  (if (== (`BTFunctionLibrary.GetBlackboardValueAsInt` (`self.BBlackboard_Direction`)) -1)
    (if (>= _returnvalue 0)
      (`BTFunctionLibrary.SetBlackboardValueAsInt` _bblackboard_direction -1)
      (`BTFunctionLibrary.SetBlackboardValueAsInt` (`self.BBlackboard_PathIndex`) _returnvalue)
      (`self.FinishExecute` true)
      (else
        (`BTFunctionLibrary.SetBlackboardValueAsInt` _bblackboard_direction 1)
        (`self.FinishExecute` false) ; the success is unticked
      ))
    (else
      (`self.FinishExecute` false))))