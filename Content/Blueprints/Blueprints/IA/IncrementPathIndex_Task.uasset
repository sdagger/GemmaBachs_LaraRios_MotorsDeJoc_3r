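; Behavior tree task that advances an NPC's patrol path index while its Blackboard direction is forward.
; It casts the pawn to NPC_Character2, checks the next index against the PatrolPath point count, then stores it and succeeds.
; Past that bound it flips direction to backward and fails, as it does when not heading forward.
; The bound subtracts negative one from the length, so the index can exceed the last valid point.
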(event `self.ReceiveExecuteAI`
  (params (OwnerController :type "AIController Object Reference") (ControlledPawn :type "Pawn Object Reference"))
  (bind _bblackboard_direction (`self.BBlackboard_Direction`))
  (bind _returnvalue (+ (`BTFunctionLibrary.GetBlackboardValueAsInt` (`self.BBlackboard_PathIndex`)) 1))
  (if (== (`BTFunctionLibrary.GetBlackboardValueAsInt` (`self.BBlackboard_Direction`)) 1)
    (bind _asnpc_character_2 (cast `/Game/Blueprints/IA/NPC_Character2` ControlledPawn))
    (if (<= _returnvalue (- (`KismetArrayLibrary.Array_Length` (`/Game/Blueprints/IA/PatrolPath.PathPoints` (`/Game/Blueprints/IA/NPC_Character2.PatrolPath` _asnpc_character_2))) -1))
      (`BTFunctionLibrary.SetBlackboardValueAsInt` _bblackboard_direction 1)
      (`BTFunctionLibrary.SetBlackboardValueAsInt` (`self.BBlackboard_PathIndex`) _returnvalue)
      (`self.FinishExecute` true)
      (else
        (`BTFunctionLibrary.SetBlackboardValueAsInt` _bblackboard_direction -1) ; when we reach the end of the path, change direction
        (`self.FinishExecute` false) ; the success is unticked
      ))
    (else
      (`self.FinishExecute` false))))