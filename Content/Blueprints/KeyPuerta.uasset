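; KeyPuerta is a door key actor that shows a floating text label when the player is nearby.
; The construction script fills the TextRender component from the ObjectName variable.
; Every Tick, it checks the distance to player character 0, showing the text within a fixed radius and rotating it to face the player, and hiding it otherwise.
; No pickup or door-opening logic is present in these graphs.
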(event `self.ReceiveTick`
  (params (DeltaSeconds :type "Float (single-precision)"))
  ;[1 1 1] Text instructions about how to open door
  (if (< (`KismetMathLibrary.VSize` (- (`self.K2_GetActorLocation` (`GameplayStatics.GetPlayerCharacter` 0)) (`self.K2_GetActorLocation`))) 300.0)
    (`SceneComponent.SetVisibility` (`self.TextRender`) true false)
    ;[1 1 1] text rotates when player rotates (so it's well seen
    (`SceneComponent.K2_SetWorldRotation` (`self.TextRender`) (`KismetMathLibrary.FindLookAtRotation` (`self.K2_GetActorLocation`) (`self.K2_GetActorLocation` (`GameplayStatics.GetPlayerCharacter` 0))) false false)
    (else
      (`SceneComponent.SetVisibility` (`self.TextRender`) false false))))

(fn `UserConstructionScript`
  (`TextRenderComponent.K2_SetText` (`self.TextRender`) (`self.ObjectName`)))