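; Behavior tree task that gives an NPC_Character2 the world location of its current patrol point.
; It reads the path index from the blackboard, takes that entry from the pawn's PatrolPath points and transforms it from the path actor's local space to world space.
; The result is written to the blackboard path vector and the task succeeds.
; A failed cast or missing path leaves the task without a FinishExecute call.
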(event `self.ReceiveExecuteAI`
  (params (OwnerController :type "AIController Object Reference") (ControlledPawn :type "Pawn Object Reference"))
  (bind _asnpc_character_2 (cast `/Game/Blueprints/IA/NPC_Character2` ControlledPawn))
  (bind _patrolpath (`/Game/Blueprints/IA/NPC_Character2.PatrolPath` _asnpc_character_2) ; validated get
    (:`then`
      (`BTFunctionLibrary.SetBlackboardValueAsVector` (`self.BBlackboard_PathVector`) (`KismetMathLibrary.TransformLocation` (`Actor.GetTransform` _patrolpath) (`|GetArrayItem` (`/Game/Blueprints/IA/PatrolPath.PathPoints` _patrolpath) (`BTFunctionLibrary.GetBlackboardValueAsInt` (`self.BBlackboard_PathIndex`)))))
      (`self.FinishExecute` true))
    (:`else`)))