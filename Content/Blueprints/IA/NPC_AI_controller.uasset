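; AI controller for patrolling NPCs that drives NPC_behaviourTree.
; On BeginPlay it runs the tree, then seeds the blackboard with patrol direction, a wait time and whether the controlled NPC_Character2's patrol path loops.
; AI perception updates on the ThirdPersonCharacter set the CanSeePlayer key from whether the stimulus was sensed.
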(event `self.ReceiveTick`
  (params (DeltaSeconds :type "Float (single-precision)"))
  ;[1 1 1] Lara
)

(event `self.ReceiveBeginPlay`
  (bind _returnvalue (`AIBlueprintHelperLibrary.GetBlackboard` null))
  ;[1 1 1] IA behaviour
  (`self.RunBehaviorTree` "/Game/Blueprints/IA/NPC_behaviourTree.NPC_behaviourTree")
  (bind _asnpc_character_2 (cast `/Game/Blueprints/IA/NPC_Character2` (`self.K2_GetPawn`)))
  (bind _output_get (set `self.MyPawn` _asnpc_character_2))
  (`BlackboardComponent.SetValueAsBool` (`AIBlueprintHelperLibrary.GetBlackboard` null) "PathLooping" (`/Game/Blueprints/IA/PatrolPath.IsLooping` (`/Game/Blueprints/IA/NPC_Character2.PatrolPath` _output_get)))
  (`BlackboardComponent.SetValueAsInt` _returnvalue "Direction" 1)
  (`BlackboardComponent.SetValueAsFloat` _returnvalue "WaitTime" 0.5))

(event `self.AIPerception1.OnTargetPerceptionUpdated`
  (params (Actor :type "Actor Object Reference") (Stimulus :type "AIStimulus Structure"))
  ;[1 1 1] IA behaviour
  (cast `/Game/ThirdPersonBP/Blueprints/ThirdPersonCharacter` Actor)
  (`BlackboardComponent.SetValueAsBool` (`AIBlueprintHelperLibrary.GetBlackboard` null) "CanSeePlayer" (`.bSuccessfullySensed` (break `AIStimulus` Stimulus))))

(fn `UserConstructionScript`)