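; NPC character Blueprint that takes damage, dies as a ragdoll and can hurt the player.
; Any damage lowers Health and updates the widget lifebar; at zero or below, movement stops, the mesh simulates physics and the actor is destroyed after a delay.
; Trigger overlap runs only if AttackPlayerNPC1 is already true, waits out the attack animation, clears the flag and directly reduces ThirdPersonCharacter Health.
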(event `self.ReceiveAnyDamage`
  (params (Damage :type "Float (single-precision)") (DamageType :type "DamageType Object Reference") (InstigatedBy :type "Controller Object Reference") (DamageCauser :type "Actor Object Reference"))
  ;[1 1 1] Lifebar
  (bind _output_get (set `self.Health` (- (`self.Health`) Damage)))
  (`KismetSystemLibrary.PrintString` (`KismetStringLibrary.Conv_DoubleToString` _output_get))
  (bind _asaihealth (cast `/Game/UI/AIHealth` (`WidgetComponent.GetUserWidgetObject` (`self.Widget`))))
  (`ProgressBar.SetPercent` (`/Game/UI/AIHealth.ProgressBar_58` _asaihealth) (`self.Health`))
  (if (<= (`self.Health`) 0.0)
    ;[1 1 1] Ragdoll
    (`CharacterMovementComponent.DisableMovement` (`self.CharacterMovement`))
    (`PrimitiveComponent.SetCollisionEnabled` (`self.Mesh`) "QueryAndPhysics")
    (`SkeletalMeshComponent.SetAllBodiesSimulatePhysics` (`self.Mesh`) true)
    (`SkeletalMeshComponent.SetAllBodiesPhysicsBlendWeight` (`self.Mesh`) 1.0 false)
    (`KismetSystemLibrary.Delay` 3.0)
    (`self.K2_DestroyActor`)))

(event `self.ReceiveTick`
  (params (DeltaSeconds :type "Float (single-precision)"))
  ;[1 1 1] Lifebar
)

(event `self.Trigger.OnComponentBeginOverlap`
  (params (OverlappedComponent :type "PrimitiveComponent Object Reference") (OtherActor :type "Actor Object Reference") (OtherComp :type "PrimitiveComponent Object Reference") (OtherBodyIndex :type Integer) (bFromSweep :type Boolean) (SweepResult :type "HitResult Structure (by ref)"))
  ;[1 1 1] Damage Player
  ;[1 1 1] Animation Attack
  (if (`self.AttackPlayerNPC1`)
    (set `self.AttackPlayerNPC1` true)
    (`KismetSystemLibrary.Delay` 2.4) ; the duration of the animation
    (set `self.AttackPlayerNPC1` false)
    (bind _asthird_person_character (cast `/Game/ThirdPersonBP/Blueprints/ThirdPersonCharacter` OtherActor))
    (set `/Game/ThirdPersonBP/Blueprints/ThirdPersonCharacter.Health` (- (`/Game/ThirdPersonBP/Blueprints/ThirdPersonCharacter.Health` _asthird_person_character) 0.01) _asthird_person_character)))

(fn `UserConstructionScript`)